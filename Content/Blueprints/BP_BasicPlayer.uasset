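; BP_BasicPlayer is a basic player pawn that binds input for movement, jumping and mouse look.
; Forward/back and left/right axes add movement along the actor's forward and right vectors, and the Jump action calls Jump.
; Horizontal look turns the controller yaw, while vertical look pitches the SArm component directly with relative rotation, with no clamp in the graph.
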(event Input|ActionEvents|InputActionJump
  (params (Key :type Key%20Structure :default "None"))
  ;[1 0.4722 0] Input_Binding
  ;;[1 0.9517 0] Space
  (:Pressed
    (Character|Jump)))

(event Input|AxisEvents|InputAxisForward/Back
  (params (AxisValue :type Float%20%28single-precision%29))
  ;[1 0.4722 0] Input_Binding
  ;;[1 0.9977 0] WASD
  (Pawn|Input|AddMovementInput (Transformation|GetActorForwardVector) AxisValue false))

(event Input|AxisEvents|InputAxisLeft/Right
  (params (AxisValue :type Float%20%28single-precision%29))
  ;[1 0.4722 0] Input_Binding
  ;;[1 0.9977 0] WASD
  (Pawn|Input|AddMovementInput (Transformation|GetActorRightVector) AxisValue false))

(event Input|AxisEvents|InputAxisLook_Left/Right
  (params (AxisValue :type Float%20%28single-precision%29))
  ;[1 0.4722 0] Input_Binding
  ;;[0.9966 1 0] Mouse X/Y
  ;;;[1 1 1] Look_Right/Left
  (Pawn|Input|AddControllerYawInput AxisValue))

(event Input|AxisEvents|InputAxisLook_Up/Down
  (params (AxisValue :type Float%20%28single-precision%29))
  ;[1 0.4722 0] Input_Binding
  ;;[0.9966 1 0] Mouse X/Y
  ;;;[1 1 1] Look_Up/Down
  (Transformation|AddRelativeRotation (Variables|Default|Gets_arm) (Math|Rotator|MakeRotator 0.0 AxisValue 0.0) false false))

(fn ConstructionScript)